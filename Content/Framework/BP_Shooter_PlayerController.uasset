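; Shooter player controller that creates the in-game HUD for the local player and manages session exit.
; On BeginPlay it clears widgets, shows a cached WB_IngameHUD and switches to game-only input; on possess, a delayed step hands that HUD to the BP_Hero_Quinn pawn.
; Events re-enable pawn input, start the HUD countdown, unhide the HUD, and destroy the session before returning to the main menu map.
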(event Custom|EnableAllInput
  (Input|EnableInput (Pawn|GetControlledPawn) self))

(event Custom|GameStartCountdown
  (Default|GameStartCountdown (Variables|Default|GetWB_IngameHUD)))

(event Custom|UnHide_IngameHUD
  (Widget|SetVisibility (Variables|Default|GetWB_IngameHUD) "Visible"))

(event Custom|EndClientSession
  (bind _asbp_shooter_game_instance (Utilities|Casting|CastToBP_Shooter_GameInstance (Game|GetGameInstance)))
  (Variables|/Game/Framework/BP_Shooter_GameInstance.BP_Shooter_GameInstance_C|SetMP_isPauseMenuVisible _asbp_shooter_game_instance false)
  (|DestroySession self
    (:then
      (Game|OpenLevel(byName) "MainMenu_Map"))
    (:OnFailure
      (Development|PrintString "Failed Destroy Session"))))

(event Custom|Lcl_SetHUDVar
  ;[1 1 1] PIE
  (Utilities|FlowControl|Delay 0.2)
  (bind _asbp_hero_quinn (Utilities|Casting|CastToBP_Hero_Quinn (Pawn|GetControlledPawn)))
  (Variables|/Game/Characters/BP_Hero_Quinn.BP_Hero_Quinn_C|SetWB%20Ingame%20HUD _asbp_hero_quinn (Variables|Default|GetWB_IngameHUD)))

(event EventBeginPlay
  (if (Pawn|IsLocalPlayerController)
    (Viewport|RemoveAllWidgets)
    (CallFunction|UIShowIngameHUD)
    (Input|SetInputModeGameOnly self false)
    (Variables|Default|SetbShowMouseCursor false)))

(event EventPossess
  (params (PossessedPawn :type Pawn%20Object%20Reference))
  (CallFunction|LclSetHUDVar))

(fn ConstructionScript)

(fn UIShowIngameHUD
  (Utilities|IsValid (Variables|Default|GetWB_IngameHUD)
    (:Is%20Valid
      _)
    (:Is%20Not%20Valid
      (bind _returnvalue (UserInterface|CreateWidget "/Game/Maps/Menu/WB_IngameHUD.WB_IngameHUD_C" self))
      (Variables|Default|SetWB_IngameHUD _returnvalue)))
  (UserInterface|Viewport|AddtoViewport (Variables|Default|GetWB_IngameHUD) 0)
  (return))