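; Game mode for the menus that manages connected players in the multiplayer lobby.
; On the lobby map, new players' menu controllers are tracked, given a lobby menu and set up; logouts remove them and refresh the names.
; UpdateLobby rebuilds the profile list from the controllers, copies each profile into its PlayerState, and pushes names or the selected level to every controller.
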(event Custom|UpdateLobby
  (params (PlayerNames :type Boolean) (LevelSelection :type Boolean))
  (if PlayerNames
    (Utilities|Array|Clear (Variables|Default|GetAll_PlayerProfiles))
    (for _array_element (Variables|Default|GetAllConnectedPlayers)
      (Utilities|Array|Add (Variables|Default|GetAll_PlayerProfiles) (Variables|/Game/Framework/BP_MenuController.BP_MenuController_C|GetPlayerProfile_Info _array_element))
      (bind _asbp_shooter_player_state (Utilities|Casting|CastToBP_Shooter_PlayerState (Variables|/Script/Engine.Controller|GetPlayerState _array_element)))
      (Variables|/Game/Framework/BP_Shooter_PlayerState.BP_Shooter_PlayerState_C|SetS_PlayerProfile _asbp_shooter_player_state (Variables|/Game/Framework/BP_MenuController.BP_MenuController_C|GetPlayerProfile_Info _array_element))))
  (for _array_element_2 (Variables|Default|GetAllConnectedPlayers)
    (if PlayerNames
      (Default|UpdatePlayerNames _array_element_2 (Variables|Default|GetAll_PlayerProfiles)))
    (if LevelSelection
      (Default|UpdateLevelSelection _array_element_2 (Variables|Default|GetSelectedLevelName)))))

(event EventBeginPlay)

(event EventTick
  (params (DeltaSeconds :type Float%20%28single-precision%29)))

(event EventHandleStartingNewPlayer
  (params (NewPlayer :type Player%20Controller%20Object%20Reference))
  (bind _returnvalue (Game|GetCurrentLevelName true))
  (switch string _returnvalue
    (:LobbyMenu_Map
      (bind _asbp_menu_controller (Utilities|Casting|CastToBP_MenuController NewPlayer))
      (Utilities|Array|Add (Variables|Default|GetAllConnectedPlayers) _asbp_menu_controller)
      (Default|CreateLobbyMenu _asbp_menu_controller)
      (Default|InitialSetup _asbp_menu_controller))))

(event EventOnLogout
  (params (ExitingController :type Controller%20Object%20Reference))
  (bind _asbp_menu_controller (Utilities|Casting|CastToBP_MenuController ExitingController))
  (Utilities|Array|RemoveItem (Variables|Default|GetAllConnectedPlayers) _asbp_menu_controller)
  (CallFunction|UpdateLobby true false))

(fn ConstructionScript)